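; BP_FirstTile is an endless-runner track tile that, when the player crosses its box trigger, asks the game mode for another tile, adds multiplied points and raises clamped walk speed.
; After a short delay it destroys itself and its tracked spawns, sparing activated powerups.
; SpawnObstacles, not called within this Blueprint, fills three lanes with obstacles, coins or powerups through cascading checks that each re-roll the random value.
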(event OnComponentBeginOverlap(Box)
  (params (OverlappedComponent :type Primitive%20Component%20Object%20Reference) (OtherActor :type Actor%20Object%20Reference) (OtherComp :type Primitive%20Component%20Object%20Reference) (OtherBodyIndex :type Integer) (bFromSweep :type Boolean) (SweepResult :type Hit%20Result%20Structure%20%28by%20ref%29))
  (Utilities|Casting|CastToBP_ThirdPersonCharacter OtherActor)
  (CallFunction|SpawnNext)
  (CallFunction|PointCounter)
  (CallFunction|SpeedIncrease)
  (Utilities|FlowControl|Delay 0.3)
  (CallFunction|DestroyChilder))

(event EventBeginPlay)

(event Collision|EventActorBeginOverlap
  (params (OtherActor :type Actor%20Object%20Reference)))

(event EventTick
  (params (DeltaSeconds :type Float%20%28single-precision%29)))

(fn ConstructionScript)

(fn SpawnObstacles
  (bind _returnvalue (Math|Random|RandomFloatinRange 0.0 1.0))
  (bind _index (Utilities|FlowControl|ForLoopwithBreak 0 2)
    (:LoopBody
      (if (Math|Float|InRange(Float) _returnvalue 0.0 0.4)
        (bind _returnvalue_2 (Game|SpawnActorfromClass "/Game/RunnerFiles/Blueprints/BP_Obstacle_Pipe.BP_Obstacle_Pipe_C" (Transformation|GetWorldTransform (Utilities|Select :Index _index :Option%200 (Variables|Default|GetLane0) :Option%201 (Variables|Default|GetLane1) :Option%202 (Variables|Default|GetLane2))) "Undefined" 0 0))
        (CallFunction|AddtoArray _returnvalue_2)
        (elif (Math|Float|InRange(Float) _returnvalue 0.4 0.5)
          (bind _returnvalue_3 (Game|SpawnActorfromClass "/Game/RunnerFiles/Blueprints/BP_Obstacle_Box.BP_Obstacle_Box_C" (Transformation|GetWorldTransform (Utilities|Select :Index _index :Option%200 (Variables|Default|GetLane0) :Option%201 (Variables|Default|GetLane1) :Option%202 (Variables|Default|GetLane2))) "Undefined" 0 0))
          (CallFunction|AddtoArray _returnvalue_3)
          (elif (Math|Float|InRange(Float) _returnvalue 0.5 0.9)
            (bind _returnvalue_4 (Game|SpawnActorfromClass "/Game/RunnerFiles/Blueprints/BP_CoinPickup.BP_CoinPickup_C" (Transformation|GetWorldTransform (Utilities|Select :Index _index :Option%200 (Variables|Default|GetLane0) :Option%201 (Variables|Default|GetLane1) :Option%202 (Variables|Default|GetLane2))) "Undefined" 0 0))
            (CallFunction|AddtoArray _returnvalue_4)
            (elif (Math|Float|InRange(Float) _returnvalue 0.9 0.97)
              (bind _returnvalue_5 (Game|SpawnActorfromClass "/Game/RunnerFiles/Blueprints/BP_MagnetPickup.BP_MagnetPickup_C" (Transformation|GetWorldTransform (Utilities|Select :Index _index :Option%200 (Variables|Default|GetLane0) :Option%201 (Variables|Default|GetLane1) :Option%202 (Variables|Default|GetLane2))) "Undefined" 0 0))
              (CallFunction|AddtoArray _returnvalue_5)
              (elif (Math|Float|InRange(Float) _returnvalue 0.97 1.0)
                (bind _returnvalue_6 (Game|SpawnActorfromClass "/Game/RunnerFiles/Blueprints/BP_BootsPickup.BP_BootsPickup_C" (Transformation|GetWorldTransform (Utilities|Select :Index _index :Option%200 (Variables|Default|GetLane0) :Option%201 (Variables|Default|GetLane1) :Option%202 (Variables|Default|GetLane2))) "Undefined" 0 0))
                (CallFunction|AddtoArray _returnvalue_6)))))))))

(fn PointCounter
  (bind _asbp_third_person_game_mode (Utilities|Casting|CastToBP_ThirdPersonGameMode (Game|GetGameMode)))
  (Variables|/Game/ThirdPerson/Blueprints/BP_ThirdPersonGameMode.BP_ThirdPersonGameMode_C|SetCurrentPoints _asbp_third_person_game_mode (+ (Variables|/Game/ThirdPerson/Blueprints/BP_ThirdPersonGameMode.BP_ThirdPersonGameMode_C|GetCurrentPoints _asbp_third_person_game_mode) (* 1 (Variables|/Game/ThirdPerson/Blueprints/BP_ThirdPersonGameMode.BP_ThirdPersonGameMode_C|GetPointsMultiplier _asbp_third_person_game_mode)))))

(fn SpawnNext
  (bind _asbp_third_person_game_mode (Utilities|Casting|CastToBP_ThirdPersonGameMode (Game|GetGameMode)))
  (Default|SpawnTile _asbp_third_person_game_mode))

(fn SpeedIncrease
  (bind _asbp_third_person_character (Utilities|Casting|CastToBP_ThirdPersonCharacter (Game|GetPlayerCharacter 0)))
  (Variables|/Script/Engine.CharacterMovementComponent|SetMaxWalkSpeed (Variables|/Script/Engine.Character|GetCharacterMovement _asbp_third_person_character) (Math|Float|Clamp(Float) (* (Variables|/Script/Engine.CharacterMovementComponent|GetMaxWalkSpeed (Variables|/Script/Engine.Character|GetCharacterMovement _asbp_third_person_character)) 1.01) 6e+02 1.2e+03)))

(fn AddtoArray
  (params (toAdd :type Actor%20Object%20Reference))
  (Utilities|Array|Add (Variables|Default|GetSpawnable) toAdd))

(fn DestroyChilder
  (for _index (range 0 (Utilities|Array|LastIndex (Variables|Default|GetSpawnable)))
    (if (Utilities|IsValid (Utilities|Array|Get(acopy) (Variables|Default|GetSpawnable) _index))
      (bind _asbp_powerup_base (Utilities|Casting|CastToBP_PowerupBase (Utilities|Array|Get(acopy) (Variables|Default|GetSpawnable) _index))
        (:then
          (if (not (Variables|/Game/RunnerFiles/Blueprints/BP_PowerupBase.BP_PowerupBase_C|GetisActivated _asbp_powerup_base))
            (Actor|DestroyActor _asbp_powerup_base)))
        (:CastFailed
          (Actor|DestroyActor (Utilities|Array|Get(acopy) (Variables|Default|GetSpawnable) _index))))))
  (Actor|DestroyActor))